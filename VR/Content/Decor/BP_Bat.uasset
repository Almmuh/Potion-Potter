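; BP_Bat is a decorative pixel bat whose eyes randomly show or hide.
; On BeginPlay it creates one dynamic instance of M_PixelBat and shares it across its three plane meshes.
; A looping one-second timer sets the EyeOpacity parameter to a random 0 or 1, so the eyes blink irregularly and in sync on all planes.
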(event Custom|ChangeEye
  (Rendering|Material|SetScalarParameterValue (Variables|Default|GetMat) "EyeOpacity" (Math|Conversions|ToFloat(Integer) (Math|Random|RandomInteger 2)) :!class /Script/Engine.MaterialInstanceDynamic))

(event EventBeginPlay
  (bind _returnvalue (Rendering|Material|CreateDynamicMaterialInstance "/Game/PixelAssets/M_PixelBat.M_PixelBat" "None" "None" :!class /Script/Engine.KismetMaterialLibrary))
  (Variables|Default|SetMat _returnvalue)
  (Utilities|Time|SetTimerbyEvent (delegate Custom|ChangeEye) 1.0 true)
  (Rendering|Material|SetMaterial (Variables|Default|GetPlane1) 0 (Variables|Default|GetMat))
  (Rendering|Material|SetMaterial (Variables|Default|GetPlane) 0 (Variables|Default|GetMat))
  (Rendering|Material|SetMaterial (Variables|Default|GetPlane2) 0 (Variables|Default|GetMat)))

(fn ConstructionScript)