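; BP_Bottle2 is a bottle actor that takes on a blend's material and moves away on reaching a collection object, driven by its Box overlap.
; Overlapping a BP_Blend copies the Blend component's material onto the Cone and moves the Cone to a hardcoded world position.
; Overlapping a BP_Collection plays a Timeline that lerps the actor from its current location toward a fixed, high-up point.
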(event OnComponentBeginOverlap(Box)
  (params (OverlappedComponent :type Primitive%20Component%20Object%20Reference) (OtherActor :type Actor%20Object%20Reference) (OtherComp :type Primitive%20Component%20Object%20Reference) (OtherBodyIndex :type Integer) (bFromSweep :type Boolean) (SweepResult :type Hit%20Result%20Structure%20%28by%20ref%29))
  (Utilities|FlowControl|Sequence
    (:then_0
      ;[1 1 1] Bottle
      (bind _asbp_blend (Utilities|Casting|CastToBP_Blend OtherActor))
      (Rendering|Material|SetMaterial (Variables|Default|GetCone) 0 (Rendering|Material|GetMaterial (Variables|/Game/Game/BP/BP_Blend.BP_Blend_C|GetBlend _asbp_blend) 0))
      (Transformation|SetWorldTransform (Variables|Default|GetCone) (Math|Transform|MakeTransform "-18.000000,152.000000,200.000000" "0, 0, 0" (Transformation|GetWorldScale (Variables|Default|GetCone))) false false))
    (:then_1
      (Utilities|Casting|CastToBP_Collection OtherActor)
      (if true
        (bind _newtrack_0 (Timeline|Timeline Play)
          (:Update
            (Transformation|SetActorLocation (Math|Vector|Lerp(Vector) (Transformation|GetActorLocation) "-314.000000,72.000000,2000.000000" _newtrack_0) false false)))))))

(fn ConstructionScript)