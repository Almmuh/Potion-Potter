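; BP_TaskBat is a task bat actor that flies from its placed location to the task spawner.
; On BeginPlay it records its own location as the start, takes the location of the BP_TaskSpawner it finds as the target, and plays a Timeline.
; Each Timeline update lerps the actor between the two points without sweeping.
; A Flytoboard event can also play the same flight.
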(event Custom|Fly%20to%20board
  (bind _newtrack_0 (Timeline|Timeline Play)
    (:Update
      (Transformation|SetActorLocation (Math|Vector|Lerp(Vector) (Variables|Default|GetStart) (Variables|Default|GetOrder%20Location) _newtrack_0) false false))))

(event EventBeginPlay
  (Variables|Default|SetStart (Transformation|GetActorLocation))
  (bind _returnvalue (Actor|GetActorOfClass "/Game/Tasks/BP_TaskSpawner.BP_TaskSpawner_C"))
  (Variables|Default|SetOrder%20Location (Transformation|GetActorLocation _returnvalue))
  (bind _newtrack_0 (Timeline|Timeline Play)
    (:Update
      (Transformation|SetActorLocation (Math|Vector|Lerp(Vector) (Variables|Default|GetStart) (Variables|Default|GetOrder%20Location) _newtrack_0) false false))))

(fn ConstructionScript)