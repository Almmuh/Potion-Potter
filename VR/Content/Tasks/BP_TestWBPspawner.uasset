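; Test spawner that creates task orders when a BP_TaskBat overlaps its box, destroying the bat.
; Each order creates a WBP_Tasks widget and advances a counter; the first four steps show it on a new widget component, later ones only print.
; Easy randomly reveals Red or Blue, weighted toward Blue, then the matching task flag is set and the icon collapses after a delay.
; Medium and Hard are empty stubs.
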(event OnComponentBeginOverlap(Box)
  (params (OverlappedComponent :type Primitive%20Component%20Object%20Reference) (OtherActor :type Actor%20Object%20Reference) (OtherComp :type Primitive%20Component%20Object%20Reference) (OtherBodyIndex :type Integer) (bFromSweep :type Boolean) (SweepResult :type Hit%20Result%20Structure%20%28by%20ref%29))
  (bind _asbp_task_bat (Utilities|Casting|CastToBP_TaskBat OtherActor))
  (Actor|DestroyActor _asbp_task_bat)
  (Development|PrintString "board")
  (CallFunction|CreateOrder))

(event Custom|CreateOrder
  (bind _task (Variables|Default|GetTask))
  (if (Utilities|IsValid _task)
    (Widget|RemovefromParent _task))
  ;[1 1 1] Sequence
  (bind _returnvalue (UserInterface|CreateWidget "/Game/Tasks/WBP_Tasks.WBP_Tasks_C"))
  (bind _result (Math|Integer|IncrementInt (Variables|Default|GetSequence))
    (:%20%20
      (switch int _result
        (:1
          (Development|PrintString "1")
          (CallFunction|Easy :!label _label)
          (bind _returnvalue_2 (AddComponent|AddWidgetComponent false (Math|Transform|MakeTransform "0, 0, 0" "0, 0, 0" "0.100000,0.150000,0.250000")))
          (UserInterface|SetWidget _returnvalue_2 _returnvalue)
          (Utilities|FlowControl|Sequence
            (:then_0
              ;[1 1 1] Red
              (if (Widget|IsVisible (Variables|/Game/Tasks/WBP_Tasks.WBP_Tasks_C|GetRed _returnvalue))
                (Variables|Default|SetRedTask true)
                (Utilities|FlowControl|Delay 1.0)
                (CallFunction|Red)))
            (:then_1
              ;[1 1 1] Blue
              (if (Widget|IsVisible (Variables|/Game/Tasks/WBP_Tasks.WBP_Tasks_C|GetBlue _returnvalue))
                (Variables|Default|SetBlueTask true)
                (Utilities|FlowControl|Delay 1.0)
                (CallFunction|Blue)))))
        (:2
          (Development|PrintString "2")
          (goto _label))
        (:3
          (Development|PrintString "3")
          (goto _label))
        (:4
          (Development|PrintString "4")
          (goto _label))
        (:5
          (Development|PrintString "5"))
        (:6
          (Development|PrintString "6"))
        (:7
          (Development|PrintString "7"))
        (:8
          (Development|PrintString "8"))))))

(event Custom|Blue
  ;[1 1 1] Blue
  (Widget|SetVisibility (Variables|/Game/Tasks/WBP_Tasks.WBP_Tasks_C|GetBlue (stale Custom|CreateOrder _returnvalue)) "Collapsed"))

(event Custom|Easy
  ;[1 1 1] Easy Randomizer
  (switch int (Math|Random|RandomIntegerinRange 1 8)
    (:1
      (Widget|SetVisibility (Variables|/Game/Tasks/WBP_Tasks.WBP_Tasks_C|GetRed (stale Custom|CreateOrder _returnvalue)) "Visible" :!label _label)
      (Development|PrintString "Easy1"))
    (:2
      (goto _label))
    (:3
      (goto _label))
    (:4
      (Widget|SetVisibility (Variables|/Game/Tasks/WBP_Tasks.WBP_Tasks_C|GetBlue (stale Custom|CreateOrder _returnvalue)) "Visible" :!label _label_2)
      (Development|PrintString "Easy2"))
    (:5
      (goto _label_2))
    (:6
      (goto _label_2))
    (:7
      (goto _label_2))
    (:8
      (goto _label_2))))

(event Custom|Medium)

(event Custom|Hard)

(event Custom|Red
  ;[1 1 1] Red
  (Widget|SetVisibility (Variables|/Game/Tasks/WBP_Tasks.WBP_Tasks_C|GetRed (stale Custom|CreateOrder _returnvalue)) "Collapsed"))

(fn ConstructionScript)