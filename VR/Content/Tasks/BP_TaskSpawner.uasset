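; BP_TaskSpawner turns an arriving task bat into a potion order shown on a task board in the VR game.
; When a BP_TaskBat overlaps its Box, it destroys the bat and calls CreateOrder.
; CreateOrder builds a WBP_TaskBoard from VRGameState's RandomTask colour, labels it with RGB values and a random name, then sets it on the Widget component.
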(event OnComponentBeginOverlap(Box)
  (params (OverlappedComponent :type Primitive%20Component%20Object%20Reference) (OtherActor :type Actor%20Object%20Reference) (OtherComp :type Primitive%20Component%20Object%20Reference) (OtherBodyIndex :type Integer) (bFromSweep :type Boolean) (SweepResult :type Hit%20Result%20Structure%20%28by%20ref%29))
  ;[1 1 1] Check when task bat collides so we can destroy it and create an order
  (bind _asbp_task_bat (Utilities|Casting|CastToBP_TaskBat OtherActor))
  (Actor|DestroyActor _asbp_task_bat)
  (CallFunction|CreateOrder))

(event Custom|CreateOrder
  ;[1 1 1] Create order and set the tasked potion
  (bind _asvrgame_state (Utilities|Casting|CastToVRGameState (Game|GetGameState)))
  (bind _returnvalue (UserInterface|CreateWidget "/Game/Tasks/WBP_TaskBoard.WBP_TaskBoard_C"))
  (Variables|/Game/Tasks/WBP_TaskBoard.WBP_TaskBoard_C|SetPotionColour _returnvalue (Variables|/Game/Tyler/VRGameState.VRGameState_C|GetRandomTask _asvrgame_state))
  (Variables|/Game/Tasks/WBP_TaskBoard.WBP_TaskBoard_C|SetBottomText _returnvalue (Utilities|Text|ToText(String) (Utilities|String|Append (Utilities|String|Append "R" (Utilities|String|ToString(Integer) (Class|KismetMathLibrary|ToInt64(Float) (.X (Math|Vector|BreakVector (Variables|/Game/Tyler/VRGameState.VRGameState_C|GetRandomTask _asvrgame_state)))))) (Utilities|String|Append " G" (Utilities|String|ToString(Integer) (Class|KismetMathLibrary|ToInt64(Float) (.Y (Math|Vector|BreakVector (Variables|/Game/Tyler/VRGameState.VRGameState_C|GetRandomTask _asvrgame_state)))))) (Utilities|String|Append " B" (Utilities|String|ToString(Integer) (Class|KismetMathLibrary|ToInt64(Float) (.Z (Math|Vector|BreakVector (Variables|/Game/Tyler/VRGameState.VRGameState_C|GetRandomTask _asvrgame_state)))))))))
  (Variables|/Game/Tasks/WBP_TaskBoard.WBP_TaskBoard_C|SetTopText _returnvalue (Utilities|Select :Index (Math|Random|RandomInteger 12) :Option%200 "Tyler" :Option%201 "Charlie" :Option%202 "Muhannad" :Option%203 "Lorna" :Option%204 "William" :Option%205 "Richard" :Option%206 "Matilda" :Option%207 "Elanor" :Option%208 "Nuno" :Option%209 "Otto" :Option%2010 "Conrad" :Option%2011 "Emery" :Option%2012 "Sylvia"))
  (UserInterface|SetWidget (Variables|Default|GetWidget) _returnvalue))

(fn ConstructionScript)