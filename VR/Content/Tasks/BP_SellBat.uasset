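; BP_SellBat is a VR task actor whose bat flies to an item sell location, then on to a far-away point.
; BeginPlay caches the VR player controller and chains two timelines that lerp the actor between these points, destroying it when the second finishes.
; Tick rotates the TaskBat component toward the player controller's location, with a yaw offset.
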(event EventTick
  (params (DeltaSeconds :type Float%20%28single-precision%29))
  (bind _as_template_vr_player_controller (Variables|Default|GetAs%20Template%20VR%20Player%20Controller))
  (bind _defaultsceneroot (Variables|Default|GetDefaultSceneRoot))
  (bind _returnvalue (Transformation|GetWorldLocation _defaultsceneroot))
  (bind _returnvalue_2 (Transformation|GetActorLocation _as_template_vr_player_controller))
  (bind _returnvalue_3 (Math|Rotator|FindLookatRotation _returnvalue _returnvalue_2))
  (Transformation|SetWorldRotation (Variables|Default|GetTaskBat) (Math|Rotator|MakeRotator (.roll _returnvalue_3) (.pitch _returnvalue_3) (+ (.yaw _returnvalue_3) 9e+01)) false false))

(event EventBeginPlay
  (bind _astemplate_vr_player_controller (Utilities|Casting|CastToTemplate_VR_Player_Controller (Game|GetPlayerController 0)))
  (Variables|Default|SetAs%20Template%20VR%20Player%20Controller _astemplate_vr_player_controller)
  (Variables|Default|SetStart (Transformation|GetWorldLocation (Variables|Default|GetTaskBat)))
  (bind _newtrack_0 (Timeline|Timeline Play)
    (:Update
      (Transformation|SetActorLocation (Math|Vector|Lerp(Vector) (Variables|Default|GetStart) (Variables|Default|GetItemSellLocation) _newtrack_0) false false))
    (:Finished
      (bind _newtrack_0_2 (Timeline|Timeline_0 Play)
        (:Update
          (Transformation|SetActorLocation (Math|Vector|Lerp(Vector) (Variables|Default|GetItemSellLocation) (Variables|Default|GetFarAwayLocation) _newtrack_0_2) false false))
        (:Finished
          (Actor|DestroyActor))))))

(fn ConstructionScript)