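; BP_PostProcessingChange cycles the game's post-processing look between a pixel effect, a pixel black-and-white effect and no effect.
; Each ChangePost call hides the PixelPost, PixelBWPost and Nopost components, then shows the one selected by PostIndex.
; The index wraps to zero at PostIndexMax, prints as a "Post Mode" debug message and increments for the next call.
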(event Custom|ChangePost
  (Rendering|SetVisibility (Variables|Default|GetPixelBWPost) false false)
  (Rendering|SetVisibility (Variables|Default|GetPixelPost) false false)
  (Rendering|SetVisibility (Variables|Default|GetNopost) false false)
  (if (== (Variables|Default|GetPostIndex) (Variables|Default|GetPostIndexMax))
    (Variables|Default|SetPostIndex 0))
  (Rendering|SetVisibility (Utilities|Select :Index (Variables|Default|GetPostIndex) :Option%200 (Variables|Default|GetPixelPost) :Option%201 (Variables|Default|GetPixelBWPost) :Option%202 (Variables|Default|GetNopost)) true false)
  (Development|PrintString (Utilities|String|Append "Post Mode " (Utilities|String|ToString(Integer) (Variables|Default|GetPostIndex))))
  (Math|Integer|IncrementInt (Variables|Default|GetPostIndex)))

(fn ConstructionScript)