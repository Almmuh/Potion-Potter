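; Potion-mixing vessel that blends the colours of ingredients dropped into it and fills potion bottles with the result.
; Tagged ingredients receive a message on overlap and are destroyed; ReturnIngreedentValue adds colours to WaterColour, which drives a dynamic material on the Cylinder.
; Tagged bottles receive the mixed colour, then the water colour resets.
; Fire, splash and bubbling sounds accompany these states, with bubbles stopped on bottle fill.
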(event Collision|EventActorBeginOverlap
  (params (OtherActor :type Actor%20Object%20Reference))
  (if (Actor|ActorHasTag OtherActor "Ingreedent")
    (Class|BPICauldron|GetIngreedentValue(Message) OtherActor self)
    (Actor|DestroyActor OtherActor)
    (Audio|SpawnSoundatLocation "/Game/Audio/water-splash-102492.water-splash-102492" (Transformation|GetWorldLocation (Variables|Default|GetCylinder)) "0, 0, 0" 1.0 1.0 0.0 "/Game/NewSoundAttenuation.NewSoundAttenuation" 0)
    (Utilities|IsValid (Variables|Default|GetWaterBubbles)
      (:Is%20Not%20Valid
        (bind _returnvalue (Audio|SpawnSoundatLocation "/Game/Audio/water-bubbles-257594.water-bubbles-257594" (Transformation|GetWorldLocation (Variables|Default|GetCylinder)) "0, 0, 0" 1.0 1.0 0.0 "/Game/NewSoundAttenuation.NewSoundAttenuation" 0))
        (Variables|Default|SetWaterBubbles _returnvalue)))
    (elif (Actor|ActorHasTag OtherActor "PotionBottle")
      (Class|BPIPotionBottle|FillPotion(Message) OtherActor (Variables|Default|GetWaterColour))
      (Variables|Default|SetWaterColour "0, 0, 0")
      (Rendering|Material|SetVectorParameterValue (Variables|Default|GetDynamicMaterial) "Colour" (Math|Color|MakeColor 0.0 0.0 0.0) :!class /Script/Engine.MaterialInstanceDynamic)
      (Audio|Components|Audio|Stop (Variables|Default|GetWaterBubbles))
      (Audio|SpawnSoundatLocation "/Game/Audio/water-splash-102492.water-splash-102492" (Transformation|GetWorldLocation (Variables|Default|GetCylinder)) "0, 0, 0" 1.0 1.0 0.0 "/Game/NewSoundAttenuation.NewSoundAttenuation" 0)
      (else
        (Development|PrintString "BP_ITEMDETECTION I have no idea what i just collided with")))))

(event EventReturnIngreedentValue
  (params (Colour :type Vector :default "0, 0, 0"))
  (Variables|Default|SetWaterColour (+ Colour (Variables|Default|GetWaterColour)))
  (Rendering|Material|SetVectorParameterValue (Variables|Default|GetDynamicMaterial) "Colour" (Math|Color|MakeColor (.x (Variables|Default|GetWaterColour)) (.y (Variables|Default|GetWaterColour)) (.z (Variables|Default|GetWaterColour))) :!class /Script/Engine.MaterialInstanceDynamic))

(event EventBeginPlay
  (bind _returnvalue (Rendering|Material|CreateDynamicMaterialInstance (Variables|Default|GetCylinder) 0 "/Game/Tyler/M_PotionColourMaster.M_PotionColourMaster" "None" :!class /Script/Engine.PrimitiveComponent))
  (Variables|Default|SetDynamicMaterial _returnvalue)
  (Audio|SpawnSoundatLocation "/Game/StarterContent/VRTemplate/Audio/Fire01.Fire01" (Transformation|GetWorldLocation (Variables|Default|GetCylinder)) "0, 0, 0" 1.0 1.0 0.0 "/Game/NewSoundAttenuation.NewSoundAttenuation" 0))

(fn ConstructionScript)