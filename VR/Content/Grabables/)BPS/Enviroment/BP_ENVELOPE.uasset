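; BP_ENVELOPE is a grabbable envelope prop that implements a VR grip interface with fixed return values.
; It uses a physics-based interactive collision grip with always-on late updates, single grip only, no secondary grip, and teleports all components.
; It exposes no grip slots, sockets or scripts, does not simulate on drop, and always reports not held.
; The event graph and construction script contain no logic.
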(event EventBeginPlay)

(event Collision|EventActorBeginOverlap
  (params (OtherActor :type Actor%20Object%20Reference)))

(event EventTick
  (params (DeltaSeconds :type Float%20%28single-precision%29)))

(fn ConstructionScript)

(fn AdvancedGripSettings
  (return ""))

(fn AllowsMultipleGrips
  (return false))

(fn ClosestGripSlotinRange
  (params (WorldLocation :type Vector :default "0, 0, 0") (bSecondarySlot :type Boolean) (CallingController :type Grip%20Motion%20Controller%20Component%20Object%20Reference) (OverridePrefix :type Name :default "None"))
  (return false "" "None"))

(fn DenyGripping
  (params (GripInitiator :type Grip%20Motion%20Controller%20Component%20Object%20Reference))
  (return false))

(fn GetGripScripts
  (return 0 false))

(fn GetGripStiffnessandDamping
  (return 0.0 0.0))

(fn GetPrimaryGripType
  (params (bIsSlot :type Boolean))
  (return "InteractiveCollisionWithPhysics"))

(fn GripBreakDistance
  (return 0.0))

(fn GripLateUpdateSetting
  (return "LateUpdatesAlwaysOn"))

(fn GripMovementReplicationType
  (return "KeepOriginalMovement"))

(fn IsHeld
  (return 0 false))

(fn RequestsSocketing
  (return 0 "None" "" false))

(fn SecondaryGripType
  (return "SG_None"))

(fn SimulateonDrop
  (return false))

(fn TeleportBehavior
  (return "TeleportAllComponents"))